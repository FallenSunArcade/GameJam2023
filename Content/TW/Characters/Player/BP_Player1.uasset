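; BP_Player1 is the player character Blueprint, linking gameplay events to the on-screen HUD and the Dead Eye slow-motion effect.
; BeginPlay creates W_HUD, then gunfire, damage and aiming events forward ammo, health and crosshair state to it.
; Dead Eye events switch global time dilation to slow motion and back, updating the HUD timer and printing the current time for debugging.
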(event EventBeginPlay
  (bind _returnvalue (UserInterface|CreateWidget "/Game/TW/UMG/W_HUD.W_HUD_C"))
  (bind _output_get (Variables|Default|SetHUDWidget _returnvalue))
  (UserInterface|Viewport|AddtoViewport _output_get 0))

(event Collision|EventActorBeginOverlap
  (params (OtherActor :type Actor%20Object%20Reference)))

(event EventTick
  (params (DeltaSeconds :type Float%20%28single-precision%29)))

(event EventGunWasFired
  (params (CurrentGunsAmmo :type Integer))
  (bind _hudwidget (Variables|Default|GetHUDWidget))
  (Utilities|IsValid _hudwidget
    (:Is%20Valid
      (Default|AmmoChangeEvent _hudwidget CurrentGunsAmmo))))

(event EventPlayerWasDamaged
  (params (PlayersCurrentHealth :type Integer))
  (bind _hudwidget (Variables|Default|GetHUDWidget))
  (Utilities|IsValid _hudwidget
    (:Is%20Valid
      (Default|HealthChangeEvent _hudwidget PlayersCurrentHealth))))

(event EventDeadEyeinProgress
  (params (CurrentTime :type Integer))
  (Utilities|Time|SetGlobalTimeDilation 0.1)
  (Default|DeadeyeEvent (Variables|Default|GetHUDWidget) true CurrentTime (Variables|Default|GetMaxDeadEyeTime))
  (Development|PrintString (Utilities|String|ToString(Integer) CurrentTime)))

(event EventDeadEyeEnded
  (params (CurrentTime :type Integer))
  (Utilities|Time|SetGlobalTimeDilation 1.0)
  (Default|DeadeyeEvent (Variables|Default|GetHUDWidget) false CurrentTime (Variables|Default|GetMaxDeadEyeTime))
  (Development|PrintString (Utilities|String|ToString(Integer) CurrentTime)))

(event EventIsPlayerAiming
  (params (bAiming :type Boolean))
  (Default|CrosshairEvent (Variables|Default|GetHUDWidget) bAiming))

(fn ConstructionScript)