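; Game mode that manages enemy spawning and keeps a running count of enemies against a limit.
; On BeginPlay it caches every SpawnPoint actor and tells each one to add an enemy.
; Event_UpdateEnemyCount applies a change to the count and, while it is below the limit, has one random spawner add an enemy and increments the count.
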(event Custom|Event_UpdateEnemyCount
  (params (value :type Integer))
  (Variables|Default|SetEnemyCount (+ (Variables|Default|GetEnemyCount) value))
  (if (< (Variables|Default|GetEnemyCount) (Variables|Default|GetEnemyLimit))
    (Default|EventAddEnemy (.OutItem (Utilities|Array|Random (Variables|Default|GetEnemySpawners))))
    (Variables|Default|SetEnemyCount (+ (Variables|Default|GetEnemyCount) 1))))

(event EventBeginPlay
  (bind _outactors (Actor|GetAllActorsOfClass "/Game/TW/Core/Spawners/SpawnPoint.SpawnPoint_C"))
  (bind _output_get (Variables|Default|SetEnemySpawners _outactors))
  (Default|EventAddEnemy _output_get))

(event EventTick
  (params (DeltaSeconds :type Float%20%28single-precision%29)))

(fn ConstructionScript)